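; Mirror Blueprint for the house that shows its planar reflection only while the player is in one of the first-floor bathrooms.
; Every Tick it casts the player character to MainChar_BP and reads its CurrentLocation enum, compared as a string.
; It then toggles the PlanarReflection component's visibility, presumably to limit the cost of planar reflections.
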(event EventBeginPlay)

(event Collision|EventActorBeginOverlap
  (params (OtherActor :type Actor%20Object%20Reference)))

(event EventTick
  (params (DeltaSeconds :type Float%20%28single-precision%29))
  (bind _planarreflection (Variables|Default|GetPlanarReflection))
  (bind _asmain_char_bp (Utilities|Casting|CastToMainChar_BP (Game|GetPlayerCharacter 0)))
  (if (or (Utilities|Enum|Equal(Enum) (Utilities|String|EnumtoString (Variables|/Script/FollowInstructions.FollowInstructionsCharacter|GetCurrentLocation _asmain_char_bp)) "FirstFloorBathroom1") (Utilities|Enum|Equal(Enum) (Utilities|String|EnumtoString (Variables|/Script/FollowInstructions.FollowInstructionsCharacter|GetCurrentLocation _asmain_char_bp)) "FirstFloorBathroom2"))
    (Rendering|SetVisibility _planarreflection true false)
    (else
      (Rendering|SetVisibility _planarreflection false false))))

(fn ConstructionScript)