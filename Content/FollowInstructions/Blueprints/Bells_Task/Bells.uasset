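; Bells task actor that detects when the player interacts with one of four bells.
; Every Tick it casts the player character to MainChar_BP and polls its Interact state, comparing the interacted object against each bell.
; A BellPlayable latch allows one trigger per interaction and resets when the player stops interacting.
; A match currently only prints that bell's name as a debug string, with no sound or sequence logic.
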(event EventBeginPlay)

(event Collision|EventActorBeginOverlap
  (params (OtherActor :type Actor%20Object%20Reference)))

(event EventTick
  (params (DeltaSeconds :type Float%20%28single-precision%29))
  (bind _asmain_char_bp (Utilities|Casting|CastToMainChar_BP (Game|GetPlayerCharacter 0)))
  (bind (_isinteracting _interactingobject) (Default|Interact _asmain_char_bp))
  (if _isinteracting
    (if (and (== _interactingobject (Variables|Default|GetBell1)) (Variables|Default|GetbellPlayable))
      (Development|PrintString "bell1")
      (Variables|Default|SetbellPlayable false :!label _label)
      (elif (and (== (Variables|Default|GetBell2) _interactingobject) (Variables|Default|GetbellPlayable))
        (Development|PrintString "bell2")
        (goto _label)
        (elif (and (Variables|Default|GetbellPlayable) (== _interactingobject (Variables|Default|GetBell3)))
          (Development|PrintString "bell3")
          (goto _label)
          (elif (and (Variables|Default|GetbellPlayable) (== _interactingobject (Variables|Default|GetBell4)))
            (Development|PrintString "bell4")
            (goto _label)))))
    (else
      (Variables|Default|SetbellPlayable true))))

(fn ConstructionScript)