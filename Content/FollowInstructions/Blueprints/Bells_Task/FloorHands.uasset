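; FloorHands is a Bells task hazard that fills a floor area with hands and slows the player inside it.
; On BeginPlay, SpawnHandsInBox adds a random number of child actors within the HandsSpawnerFloor box, randomizing position, tilt, yaw and per-axis scale.
; Overlapping the separate Box trigger lowers the player character's walk and run speeds, respecting sprint state; leaving sets hardcoded normal speeds.
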(event OnComponentBeginOverlap(Box)
  (params (OverlappedComponent :type Primitive%20Component%20Object%20Reference) (OtherActor :type Actor%20Object%20Reference) (OtherComp :type Primitive%20Component%20Object%20Reference) (OtherBodyIndex :type Integer) (bFromSweep :type Boolean) (SweepResult :type Hit%20Result%20Structure%20%28by%20ref%29))
  (bind _returnvalue (Game|GetPlayerCharacter 0))
  ;[1 1 1] Sets the players Speed once they enter or exit the collision box
  (if (== OtherActor _returnvalue)
    (Development|PrintString "in box")
    (bind _asfollow_instructions_character (Utilities|Casting|CastToFollowInstructionsCharacter _returnvalue))
    (if (Variables|/Script/FollowInstructions.FollowInstructionsCharacter|GetbIsSprinting _asfollow_instructions_character)
      (Variables|/Script/Engine.CharacterMovementComponent|SetMaxWalkSpeed (Variables|/Script/Engine.Character|GetCharacterMovement _asfollow_instructions_character) 175.0)
      (else
        (Variables|/Script/Engine.CharacterMovementComponent|SetMaxWalkSpeed (Variables|/Script/Engine.Character|GetCharacterMovement _asfollow_instructions_character) 125.0)))
    (Variables|/Script/FollowInstructions.FollowInstructionsCharacter|SetWalkSpeed _asfollow_instructions_character 125.0)
    (Variables|/Script/FollowInstructions.FollowInstructionsCharacter|SetRunSpeed _asfollow_instructions_character 175.0)))

(event OnComponentEndOverlap(Box)
  (params (OverlappedComponent :type Primitive%20Component%20Object%20Reference) (OtherActor :type Actor%20Object%20Reference) (OtherComp :type Primitive%20Component%20Object%20Reference) (OtherBodyIndex :type Integer))
  (bind _returnvalue (Game|GetPlayerCharacter 0))
  ;[1 1 1] Sets the players Speed once they enter or exit the collision box
  (if (== OtherActor _returnvalue)
    (Development|PrintString "exited box")
    (bind _asfollow_instructions_character (Utilities|Casting|CastToFollowInstructionsCharacter _returnvalue))
    (if (Variables|/Script/FollowInstructions.FollowInstructionsCharacter|GetbIsSprinting _asfollow_instructions_character)
      (Variables|/Script/Engine.CharacterMovementComponent|SetMaxWalkSpeed (Variables|/Script/Engine.Character|GetCharacterMovement _asfollow_instructions_character) 4e+02)
      (else
        (Variables|/Script/Engine.CharacterMovementComponent|SetMaxWalkSpeed (Variables|/Script/Engine.Character|GetCharacterMovement _asfollow_instructions_character) 3e+02)))
    (Variables|/Script/FollowInstructions.FollowInstructionsCharacter|SetWalkSpeed _asfollow_instructions_character 3e+02)
    (Variables|/Script/FollowInstructions.FollowInstructionsCharacter|SetRunSpeed _asfollow_instructions_character 4e+02)))

(event EventBeginPlay
  (CallFunction|SpawnHandsinBox (Variables|Default|GetHands%20Spawner_Floor) "0, 0, 0" 18 25))

(fn ConstructionScript)

(fn SpawnHandsinBox
  (params (Bounding%20Box :type Box%20Component%20Object%20Reference) (Rotation :type Rotator) (Min :type Integer) (Max :type Integer))
  (bind _returnvalue (Math|Random|RandomFloatinRange 0.75 1.1))
  (for _index (range 0 (Math|Random|RandomIntegerinRange Min Max))
    (AddComponent|AddChildActorComponent false (Math|Transform|MakeTransform (Math|Random|RandomPointinBoundingBox (Variables|/Script/Engine.SceneComponent|GetRelativeLocation Bounding%20Box) (Variables|/Script/Engine.BoxComponent|GetBoxExtent Bounding%20Box)) (Math|Rotator|CombineRotators (Math|Rotator|MakeRotator (Math|Random|RandomFloatinRange 0.0 25.0) (Math|Random|RandomFloatinRange 0.0 25.0) (Math|Random|RandomFloatinRange 0.0 3.6e+02)) Rotation) (Math|Vector|MakeVector _returnvalue _returnvalue _returnvalue)))))