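; Player cellphone Blueprint that shows an in-game clock and doubles as a flashlight.
; Every Tick it reads CurrentDateTime from the player's FollowInstructionsCharacter and writes it to the Time text as a 12-hour clock, zero-padding minutes.
; Pressing F toggles the SpotLight's visibility, but only while MainChar_BP's UsingPhone flag is set.
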(event EventBeginPlay)

(event Collision|EventActorBeginOverlap
  (params (OtherActor :type Actor%20Object%20Reference)))

(event EventTick
  (params (DeltaSeconds :type Float%20%28single-precision%29))
  (bind _time (Variables|Default|Gettime))
  ;[1 1 1] Changes time to match current time
  (bind _asfollow_instructions_character (Utilities|Casting|CastToFollowInstructionsCharacter (Game|GetPlayerCharacter 0)))
  (if (< (Class|KismetMathLibrary|GetMinute (Variables|/Script/FollowInstructions.FollowInstructionsCharacter|GetCurrentDateTime _asfollow_instructions_character)) 10)
    (Rendering|Components|TextRender|SetText _time (Utilities|Text|FormatText "{hour} : 0{min}" (Class|KismetMathLibrary|GetHour12 (Variables|/Script/FollowInstructions.FollowInstructionsCharacter|GetCurrentDateTime _asfollow_instructions_character)) (Class|KismetMathLibrary|GetMinute (Variables|/Script/FollowInstructions.FollowInstructionsCharacter|GetCurrentDateTime _asfollow_instructions_character))))
    (else
      (Rendering|Components|TextRender|SetText _time (Utilities|Text|FormatText "{hour} : {min}" (Class|KismetMathLibrary|GetHour12 (Variables|/Script/FollowInstructions.FollowInstructionsCharacter|GetCurrentDateTime _asfollow_instructions_character)) (Class|KismetMathLibrary|GetMinute (Variables|/Script/FollowInstructions.FollowInstructionsCharacter|GetCurrentDateTime _asfollow_instructions_character)))))))

(event Input|KeyboardEvents|F
  (params (Key :type Key%20Structure))
  ;[1 1 1] Using the phone Flashlight on a toggle
  (:Pressed
    (bind _asmain_char_bp (Utilities|Casting|CastToMainChar_BP (Game|GetPlayerCharacter 0)))
    (if (Variables|/Game/FollowInstructions/Blueprints/MainCharBps/MainChar_BP.MainChar_BP_C|GetUsing_Phone _asmain_char_bp)
      (Rendering|ToggleVisibility (Variables|Default|GetSpotLight) false))))

(fn ConstructionScript)