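; Instructions list Blueprint that shows the game's rules as flippable pages on a Cube mesh.
; BeginPlay fills an array with the rule materials, and Tick tracks whether the Cube is visible.
; While it is visible, the 2 key and the 1Down input action step forward and back through the array with wraparound, swapping the Cube's material to change the page.
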(event EventBeginPlay
  (bind _material_lists (Variables|Default|GetMaterial_Lists))
  ;[1 1 1] Add stuff into a material array
  (Utilities|Array|Add _material_lists "/Game/FollowInstructions/Materials/Instructions_list/INstructionsMaterials/Angel_Satue_Mat.Angel_Satue_Mat")
  (Utilities|Array|Add _material_lists "/Game/FollowInstructions/Materials/Instructions_list/INstructionsMaterials/Wall_demon_rule_Mat.Wall_demon_rule_Mat")
  (Utilities|Array|Add _material_lists "/Game/FollowInstructions/Materials/Instructions_list/INstructionsMaterials/Attic_Rule_Mat.Attic_Rule_Mat")
  (Utilities|Array|Add _material_lists "/Game/FollowInstructions/Materials/Instructions_list/INstructionsMaterials/Clock_rule_Mat.Clock_rule_Mat")
  (Utilities|Array|Add _material_lists "/Game/FollowInstructions/Materials/Instructions_list/INstructionsMaterials/TV_GeneralRule_Mat.TV_GeneralRule_Mat")
  (Utilities|Array|Add _material_lists "/Game/FollowInstructions/Materials/Instructions_list/INstructionsMaterials/TV_SpecificRule_Mat.TV_SpecificRule_Mat")
  (Utilities|Array|Add _material_lists "/Game/FollowInstructions/Materials/Instructions_list/INstructionsMaterials/Lights_Rule_Mat.Lights_Rule_Mat")
  (Utilities|Array|Add _material_lists "/Game/FollowInstructions/Materials/Instructions_list/INstructionsMaterials/Triangles_Mat.Triangles_Mat"))

(event EventTick
  (params (DeltaSeconds :type Float%20%28single-precision%29))
  ;[1 1 1] Sets a bool to true or false based on visiblity
  (if (Rendering|IsVisible (Variables|Default|GetCube))
    (Variables|Default|SetIfVisible true)
    (else
      (Variables|Default|SetIfVisible false))))

(event Input|ActionEvents|InputAction1Down
  (params (Key :type Key%20Structure))
  (bind _material_lists (Variables|Default|GetMaterial_Lists))
  ;[1 1 1] Changes the Pages of the instructions back and forth
  (:Pressed
    (if (Variables|Default|GetIfVisible)
      (Math|Integer|DecrementInt (Variables|Default|GetCurrent_PageIndex)
        (:%20%20
          (if (< (Variables|Default|GetCurrent_PageIndex) 0)
            (Variables|Default|SetCurrent_PageIndex (Utilities|Array|LastIndex _material_lists)))
          (Rendering|Material|SetMaterial (Variables|Default|GetCube) 0 (Utilities|Array|Get(acopy) _material_lists (Variables|Default|GetCurrent_PageIndex))))))))

(event Input|KeyboardEvents|2
  (params (Key :type Key%20Structure))
  (bind _material_lists (Variables|Default|GetMaterial_Lists))
  ;[1 1 1] Changes the Pages of the instructions back and forth
  (:Pressed
    (if (Variables|Default|GetIfVisible)
      (Math|Integer|IncrementInt (Variables|Default|GetCurrent_PageIndex)
        (:%20%20
          (if (> (Variables|Default|GetCurrent_PageIndex) (Utilities|Array|LastIndex _material_lists))
            (Variables|Default|SetCurrent_PageIndex 0))
          (Rendering|Material|SetMaterial (Variables|Default|GetCube) 0 (Utilities|Array|Get(acopy) _material_lists (Variables|Default|GetCurrent_PageIndex))))))))

(fn ConstructionScript)