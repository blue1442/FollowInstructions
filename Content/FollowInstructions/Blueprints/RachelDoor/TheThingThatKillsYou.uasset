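; A lethal chaser actor, described as hands, that hunts the player's MainChar_BP character and sends them to Death_level on contact.
; Each Tick it sets its rotation from the horizontal direction to the player, with a fixed rotational offset.
; It also calls MoveComponentTo on its root toward the player's location, scaling duration by distance to target a constant approach speed.
; Overlapping the player prints a taunt before loading the death level.
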(event Collision|EventActorBeginOverlap
  (params (OtherActor :type Actor%20Object%20Reference))
  (Utilities|Casting|CastToMainChar_BP OtherActor)
  (Development|PrintString "Ha HA HA")
  (Game|OpenLevel(byName) "Death_level"))

(event EventTick
  (params (DeltaSeconds :type Float%20%28single-precision%29))
  (bind _defaultsceneroot (Variables|Default|GetDefaultSceneRoot))
  ;[1 1 1] moves hands towards the player
  (bind _asmain_char_bp (Utilities|Casting|CastToMainChar_BP (Game|GetPlayerCharacter 0)))
  (Transformation|SetActorRotation (Math|Conversions|RotationFromXVector (Math|Vector|RotateVector (Math|Vector|Normalize (* (- (Transformation|GetWorldLocation (Variables|/Script/Engine.Actor|GetRootComponent _asmain_char_bp)) (Transformation|GetWorldLocation _defaultsceneroot)) "1.000000,1.000000, 0")) "0.000000,180.000000, 0")))
  (Components|MoveComponentTo _defaultsceneroot (Transformation|GetWorldLocation (Variables|/Script/Engine.Actor|GetRootComponent _asmain_char_bp)) "0, 0, 0" false false (/ (Math|Vector|Distance(Vector) (Transformation|GetWorldLocation (Variables|/Script/Engine.Actor|GetRootComponent _asmain_char_bp)) (Transformation|GetWorldLocation _defaultsceneroot)) 6e+02) false))

(fn ConstructionScript)