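; SoundMaker is an actor that plays occasional random, attenuated sounds from Rachel's room.
; Tick reads CurrentHour from MainChar_BP and permanently sets the Past8 flag once the hour equals 7, despite the flag's name.
; While flagged, each tick decrements a cooldown and rolls a rare chance to play the cue at the mesh's location.
; Each play resets the cooldown, which counts frames and so depends on frame rate.
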(event Custom|Play%20Sound
  (Audio|PlaySoundatLocation "/Game/FollowInstructions/Sounds/RachelsRoom/RachelRoomSoundCue.RachelRoomSoundCue" (Transformation|GetWorldLocation (Variables|Default|GetStaticMesh)) "0, 0, 0" 0.4 1.0 0.0 "/Game/FollowInstructions/Sounds/Rachel_room.Rachel_room" 0 0)
  (Variables|Default|SetTimer 3600))

(event EventBeginPlay)

(event Collision|EventActorBeginOverlap
  (params (OtherActor :type Actor%20Object%20Reference)))

(event EventTick
  (params (DeltaSeconds :type Float%20%28single-precision%29))
  (bind _timer (Variables|Default|GetTimer))
  (bind _asmain_char_bp (Utilities|Casting|CastToMainChar_BP (Game|GetPlayerCharacter 0)))
  (if (== (Variables|/Game/FollowInstructions/Blueprints/MainCharBps/MainChar_BP.MainChar_BP_C|GetCurrent_Hour _asmain_char_bp) 7)
    (bind _output_get (Variables|Default|SetPast8 true)))
  (if _output_get
    (Math|Integer|DecrementInt _timer
      (:%20%20
        (if (and (== (Math|Random|RandomInteger 10000) 0) (<= _timer 0))
          (CallFunction|PlaySound))))))

(fn ConstructionScript)