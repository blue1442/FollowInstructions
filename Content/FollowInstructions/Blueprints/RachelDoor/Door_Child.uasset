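; Rachel's Door, a child door Blueprint that triggers a scripted death sequence when the player opens it too far.
; Tick watches the door's relative rotation, latches FateisSealed near an angle threshold, disables player input and rotates the door incrementally until fully open.
; At that point it sets the character's LightsAreOff, and a one-shot Safeguard plays a power-down sound, hides the phone and, after a delay, spawns TheThingThatKillsYou at a hardcoded location.
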(event Collision|EventActorBeginOverlap
  (params (OtherActor :type Actor%20Object%20Reference)))

(event EventTick
  (params (DeltaSeconds :type Float%20%28single-precision%29))
  (bind _returnvalue (Game|GetPlayerCharacter 0))
  (bind _door (Variables|Default|GetDoor))
  (bind _returnvalue_2 (Transformation|GetRelativeTransform _door))
  (bind _returnvalue_3 (Math|Transform|TransformRotation _returnvalue_2 "0, 0, 0"))
  (bind _returnvalue_4 (Math|Rotator|CombineRotators _returnvalue_3 "0,1.000000, 0"))
  ;[1 1 1] You have opened Rachel's Door, remove player input and start death sequence
  (if (or (Variables|Default|GetFateisSealed) (Math|Rotator|Equal(Rotator) _returnvalue_3 "0,-45.000000, 0" 5.0))
    (Variables|Default|SetFateisSealed true)
    (Development|PrintString "Yes")
    (bind _asmain_char_bp (Utilities|Casting|CastToMainChar_BP _returnvalue))
    (Input|DisableInput _returnvalue (Game|GetPlayerController 0))
    (if (Math|Rotator|Equal(Rotator) _returnvalue_4 "0, 0, 0" 1.0)
      (Variables|/Game/FollowInstructions/Blueprints/MainCharBps/MainChar_BP.MainChar_BP_C|SetlightsAreOff _asmain_char_bp true)
      (if (Variables|Default|Getsafeguard)
        (Audio|PlaySound2D "/Game/FollowInstructions/Sounds/Power_Down_1_-_Free_Sound_Effect.Power_Down_1_-_Free_Sound_Effect" 0.68 1.0 0.0 0 0)
        (Variables|Default|Setsafeguard false)
        (if (Variables|/Script/Engine.SceneComponent|GetbVisible (Variables|/Game/FollowInstructions/Blueprints/MainCharBps/MainChar_BP.MainChar_BP_C|Getphone _asmain_char_bp))
          (Rendering|SetVisibility (Variables|/Game/FollowInstructions/Blueprints/MainCharBps/MainChar_BP.MainChar_BP_C|Getphone _asmain_char_bp) false false))
        (Utilities|FlowControl|Delay 2.0)
        (Game|SpawnActorfromClass "/Game/FollowInstructions/Blueprints/RachelDoor/TheThingThatKillsYou.TheThingThatKillsYou_C" (Math|Transform|MakeTransform "1993.796509,-1840.000000,611.049927") "Undefined" 0 0))
      (else
        ;[1 1 1] Once A certain angle threshold is reached, then continue to open the door until its fully open
        (Transformation|SetRelativeLocationAndRotation (Variables|Default|GetDoor) (Math|Transform|TransformLocation _returnvalue_2 "0, 0, 0") _returnvalue_4 false false)))))

(fn ConstructionScript
  (|CallParentFunction))