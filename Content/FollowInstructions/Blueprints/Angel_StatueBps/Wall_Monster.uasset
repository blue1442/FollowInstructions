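; Wall monster hazard that lurks at one of six preset wall spots and kills a player who lingers in its trigger.
; A Tick countdown periodically moves it to a random spot via TeleportToLocation.
; Overlap raises a frame-counted timer that drives whispering volume and decays outside the trigger.
; At the threshold it forces the player's look, disables input, then reveals and animates the demon mesh; restore and quit nodes are unwired.
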(event EventBeginPlay
  (Variables|Default|SetWallMonsterTimer 0.0)
  (Audio|Components|Audio|SetVolumeMultiplier (Variables|Default|GetWhispering) 0.01 :!class /Script/Engine.AudioComponent)
  (Variables|Default|SetTeleport%20Timer 1200)
  (Rendering|SetVisibility (Variables|Default|GetDemon_Mesh) false false))

(event Collision|EventActorBeginOverlap
  (params (OtherActor :type Actor%20Object%20Reference))
  (Utilities|Casting|CastToMainChar_BP OtherActor)
  (Variables|Default|SetIsInTrigger true))

(event EventTick
  (params (DeltaSeconds :type Float%20%28single-precision%29))
  (bind _returnvalue (Game|GetPlayerCharacter 0))
  (bind _wallmonstertimer (Variables|Default|GetWallMonsterTimer))
  (bind _whispering (Variables|Default|GetWhispering))
  (bind _demon_mesh (Variables|Default|GetDemon_Mesh))
  (bind _result (Math|Integer|DecrementInt (Variables|Default|GetTeleport%20Timer))
    (:%20%20
      (if (<= _result 0)
        (CallFunction|TeleporttoLocation))
      (if (not (Variables|Default|GetWallMonsterSpawned))
        (if (Variables|Default|GetIsInTrigger)
          (bind _result_2 (Math|Float|IncrementFloat _wallmonstertimer)
            (:%20%20
              (Audio|Components|Audio|SetVolumeMultiplier _whispering (Math|Float|Max(Float) (/ _wallmonstertimer 6e+01) 0.01) :!class /Script/Engine.AudioComponent :!label _label)
              (if (>= _result_2 3.6e+02)
                (Variables|Default|SetWallMonsterSpawned true)
                (Audio|Components|Audio|AdjustVolume _whispering 0.0 0.0 :!class /Script/Engine.AudioComponent)
                (Development|PrintString "You Have died to the wall monster")
                (bind _asmain_char_bp (Utilities|Casting|CastToMainChar_BP _returnvalue))
                (Default|PlayerLookat _asmain_char_bp self 1.0 "0, 0, 0")
                (Input|DisableInput _returnvalue (Game|GetPlayerController 0))
                (Utilities|FlowControl|Delay 3.0)
                (Rendering|SetVisibility _demon_mesh true false)
                (Timeline|Timeline_WallDemon PlayFromStart
                  (:Update
                    (Transformation|SetRelativeLocation _demon_mesh "0,10.000000, 0" false false)
                    (Components|Animation|PlayAnimation (Variables|Default|GetDemon_Mesh) "/Game/FollowInstructions/Animations/Wall_Monster_Animation_Anim_Armature_ArmatureAction_001.Wall_Monster_Animation_Anim_Armature_ArmatureAction_001" false))))))
          (elif (not (<= _wallmonstertimer 0.0))
            (Math|Float|DecrementFloat _wallmonstertimer
              (:%20%20
                (goto _label)))))))))

(event Collision|EventActorEndOverlap
  (params (OtherActor :type Actor%20Object%20Reference))
  (Utilities|Casting|CastToMainChar_BP OtherActor)
  (Variables|Default|SetIsInTrigger false))

(fn ConstructionScript)

(fn TeleporttoLocation
  (bind _defaultsceneroot (Variables|Default|GetDefaultSceneRoot))
  (switch int (Math|Random|RandomIntegerinRange 0 5)
    (:0
      (Variables|Default|SetNewTransform "609.000000,-463.000000,95.000000")
      (Variables|Default|SetNewRotation "0,180.000000, 0"))
    (:1
      (Variables|Default|SetNewTransform "1285.000000,-1020.500000,95.000000")
      (Variables|Default|SetNewRotation "0, 0, 0"))
    (:2
      (Variables|Default|SetNewTransform "1726.000000,-749.000000,95.000000")
      (Variables|Default|SetNewRotation "0,-90.000000,0.000000"))
    (:3
      (Variables|Default|SetNewTransform "2225.000000,-883.500000,127.000000")
      (Variables|Default|SetNewRotation "0,-90.000000, 0"))
    (:4
      (Variables|Default|SetNewTransform "2524.000000,-2016.500000,120.000000")
      (Variables|Default|SetNewRotation "0, 0, 0"))
    (:5
      (Variables|Default|SetNewTransform "1734.000000,-1594.000000,120.000000")
      (Variables|Default|SetNewRotation "0,-90.000000, 0")))
  (Transformation|SetWorldLocation _defaultsceneroot (Variables|Default|GetNewTransform) false false)
  (Transformation|SetWorldRotation _defaultsceneroot (Variables|Default|GetNewRotation) false false)
  (Variables|Default|SetTeleport%20Timer 3600))