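; Shadow_Demon is a self-propagating hazard that sends the player to Death_level when they overlap its KillArea.
; One second after BeginPlay it spawns another Shadow_Demon, then destroys itself ten seconds later, forming a rolling chain.
; SpawnMore randomly picks one of the N, E, S or W spawn points, with east weighted double; the D and U branches are unconnected.
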(event OnComponentBeginOverlap(killArea)
  (params (OverlappedComponent :type Primitive%20Component%20Object%20Reference) (OtherActor :type Actor%20Object%20Reference) (OtherComp :type Primitive%20Component%20Object%20Reference) (OtherBodyIndex :type Integer) (bFromSweep :type Boolean) (SweepResult :type Hit%20Result%20Structure%20%28by%20ref%29))
  (bind _asmain_char_bp (Utilities|Casting|CastToMainChar_BP (Game|GetPlayerCharacter 0)))
  (if (== _asmain_char_bp OtherActor)
    (Game|OpenLevel(byName) "Death_level")))

(event EventBeginPlay
  (Utilities|FlowControl|Delay 1.0)
  (CallFunction|SpawnMore)
  (Utilities|FlowControl|Delay 1e+01)
  (Actor|DestroyActor))

(event Collision|EventActorBeginOverlap
  (params (OtherActor :type Actor%20Object%20Reference)))

(event EventTick
  (params (DeltaSeconds :type Float%20%28single-precision%29)))

(fn ConstructionScript)

(fn SpawnMore
  (switch int (Math|Random|RandomInteger 5)
    (:0
      (bind _output_get (LocalVariables|SetNewLocation (Transformation|GetWorldTransform (Variables|Default|GetspawnPointN)) :!label _label)))
    (:1
      (LocalVariables|SetNewLocation (Transformation|GetWorldTransform (Variables|Default|GetspawnPointE)) :!label _label_2))
    (:2
      (LocalVariables|SetNewLocation (Transformation|GetWorldTransform (Variables|Default|GetspawnPointS))))
    (:3
      (goto _label_2))
    (:4
      (LocalVariables|SetNewLocation (Transformation|GetWorldTransform (Variables|Default|GetspawnPointW))))
    (:5
      (goto _label)))
  (Game|SpawnActorfromClass "Shadow_Demon_C" _output_get "Undefined" 0 0))