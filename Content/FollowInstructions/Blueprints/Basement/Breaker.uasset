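; Breaker box that triggers a 1:00 blackout with shadow demon spawns until the player returns the missing breaker.
; Tick watches the player's clock, then flags lights off, spawns the movable breaker and an initial demon wave, with a delayed safeguard reset.
; During the blackout, a frame counter drives recurring random spawns, and entering the basement triggers a one-time ambush.
; Overlapping the box with the breaker shows it installed, destroys the carried item and clears the blackout flag.
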(event OnComponentBeginOverlap(Box)
  (params (OverlappedComponent :type Primitive%20Component%20Object%20Reference) (OtherActor :type Actor%20Object%20Reference) (OtherComp :type Primitive%20Component%20Object%20Reference) (OtherBodyIndex :type Integer) (bFromSweep :type Boolean) (SweepResult :type Hit%20Result%20Structure%20%28by%20ref%29))
  ;[1 1 1] Check to see if the fuse has touched the box
  (if (== OtherActor (Variables|Default|Getmovable_breaker))
    (Rendering|SetVisibility (Variables|Default|GetBreaker3) true false)
    (bind _asmain_char_bp (Utilities|Casting|CastToMainChar_BP (Game|GetPlayerCharacter 0)))
    (Audio|PlaySoundatLocation "/Game/FollowInstructions/Sounds/Insert_Sound.Insert_Sound" (Transformation|GetWorldLocation (Variables|Default|GetStaticMesh)) "0, 0, 0" 1.5 1.0 0.0 0 0 0)
    (Default|ItemDrop _asmain_char_bp)
    (Variables|/Game/FollowInstructions/Blueprints/MainCharBps/MainChar_BP.MainChar_BP_C|SetlightsAreOff _asmain_char_bp false)
    (Actor|DestroyActor OtherActor)))

(event Custom|SpawnShadowMonsters
  ;[1 1 1] Spawns the breaker and the Shadow Demons
  (bind _asmain_char_bp (Utilities|Casting|CastToMainChar_BP (Game|GetPlayerCharacter 0)))
  (Variables|/Game/FollowInstructions/Blueprints/MainCharBps/MainChar_BP.MainChar_BP_C|SetlightsAreOff _asmain_char_bp true)
  (bind _returnvalue (Game|SpawnActorfromClass "/Game/FollowInstructions/Blueprints/Basement/Movable_Breaker.Movable_Breaker_C" (Math|Transform|MakeTransform "420.000000,-233.000000,37.000000") "Undefined" 0 0))
  (Variables|Default|Setmovable_breaker _returnvalue)
  (Audio|PlaySound2D "/Game/FollowInstructions/Sounds/Power_Down_1_-_Free_Sound_Effect.Power_Down_1_-_Free_Sound_Effect" 1.3 1.0 0.0 0 0)
  (AI|SpawnAIFromClass "/Game/FollowInstructions/Blueprints/Basement/Shadow_Demon/ShadowDemon.ShadowDemon_C" "/Game/FollowInstructions/Blueprints/Basement/Shadow_Demon/PanicBT_2.PanicBT_2" "2600.000000,-1200.000000,93.000000" "0, 0, 0" false)
  (AI|SpawnAIFromClass "/Game/FollowInstructions/Blueprints/Basement/Shadow_Demon/ShadowDemon.ShadowDemon_C" "/Game/FollowInstructions/Blueprints/Basement/Shadow_Demon/PanicBT_2.PanicBT_2" "1375.000000,-1640.000000,575.000000" "0, 0, 0" false)
  (AI|SpawnAIFromClass "/Game/FollowInstructions/Blueprints/Basement/Shadow_Demon/ShadowDemon.ShadowDemon_C" "/Game/FollowInstructions/Blueprints/Basement/Shadow_Demon/PanicBT_2.PanicBT_2" "1375.000000,-503.000000,85.000000" "0, 0, 0" false)
  (Utilities|FlowControl|Delay 5.0)
  (Variables|Default|SetSafeguard true))

(event Custom|BasementSpawn
  ;[1 1 1] Spawn Demons when enter basement
  (Development|PrintString "Spawn Shadow Demons in basement")
  (AI|SpawnAIFromClass "/Game/FollowInstructions/Blueprints/Basement/Shadow_Demon/ShadowDemon.ShadowDemon_C" "/Game/FollowInstructions/Blueprints/Basement/Shadow_Demon/PanicBT_2.PanicBT_2" "2570.000000,-1430.000000,-355.000000" "0, 0, 0" false)
  (AI|SpawnAIFromClass "/Game/FollowInstructions/Blueprints/Basement/Shadow_Demon/ShadowDemon.ShadowDemon_C" "/Game/FollowInstructions/Blueprints/Basement/Shadow_Demon/PanicBT_2.PanicBT_2" "2570.000000,-250.000000,-355.000000" "0, 0, 0" false))

(event EventTick
  (params (DeltaSeconds :type Float%20%28single-precision%29))
  ;[1 1 1] turns off the lights at X time
  (bind _result (Math|Integer|IncrementInt (Variables|Default|Gettimer))
    (:%20%20
      (bind _asmain_char_bp (Utilities|Casting|CastToMainChar_BP (Game|GetPlayerCharacter 0)))
      (if (Variables|/Game/FollowInstructions/Blueprints/MainCharBps/MainChar_BP.MainChar_BP_C|GetlightsAreOff _asmain_char_bp)
        ;;[1 1 1] Spawn Demons Overtime when the lighst are off
        (if (== (Math|Integer|%(Integer) _result 600) 0)
          (switch int (Math|Random|RandomInteger 2)
            (:Default
              (Variables|Default|SetShadowSpawn "1375.000000,-1640.000000,93.000000" :!label _label))
            (:0
              (goto _label))
            (:1
              (Variables|Default|SetShadowSpawn "2600.000000,-1200.000000,93.000000"))
            (:2
              (Variables|Default|SetShadowSpawn "1375.000000,-500.000000,85.000000")))
          (AI|SpawnAIFromClass "/Game/FollowInstructions/Blueprints/Basement/Shadow_Demon/ShadowDemon.ShadowDemon_C" "/Game/FollowInstructions/Blueprints/Basement/Shadow_Demon/PanicBT_2.PanicBT_2" (Variables|Default|GetShadowSpawn) "0, 0, 0" false)
          (else
            ;;[1 1 1] When in basement
            (if (and (Utilities|Enum|Equal(Enum) (Utilities|String|EnumtoString (Variables|/Script/FollowInstructions.FollowInstructionsCharacter|GetCurrentLocation _asmain_char_bp)) "Basement") (Variables|Default|GetSafeguard2))
              (Variables|Default|SetSafeguard2 false)
              (CallFunction|BasementSpawn))))
        (elif (Math|Boolean|ANDBoolean (== (Class|KismetMathLibrary|GetHour12 (Variables|/Script/FollowInstructions.FollowInstructionsCharacter|GetCurrentDateTime _asmain_char_bp)) 1) (Variables|Default|GetSafeguard) (== (Class|KismetMathLibrary|GetMinute (Variables|/Script/FollowInstructions.FollowInstructionsCharacter|GetCurrentDateTime _asmain_char_bp)) 0))
          (Variables|Default|SetSafeguard false)
          (CallFunction|SpawnShadowMonsters))))))

(fn ConstructionScript)