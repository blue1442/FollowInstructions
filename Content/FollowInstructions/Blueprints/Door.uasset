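; Door actor that keeps its Door component within a swing range between a closed and an open rotation.
; Each Tick adds the Door's world yaw to that of the Closed and Open reference components and checks the sign.
; A positive Closed sum snaps the Door to zero rotation; otherwise a negative Open sum snaps it to a quarter turn, using hard-coded world rotations.
; Nothing here drives the swing itself.
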(event EventBeginPlay)

(event Collision|EventActorBeginOverlap
  (params (OtherActor :type Actor%20Object%20Reference)))

(event EventTick
  (params (DeltaSeconds :type Float%20%28single-precision%29))
  (bind _door (Variables|Default|GetDoor))
  (bind _door_2 (Variables|Default|GetDoor))
  (bind _returnvalue (Transformation|GetWorldRotation _door_2))
  (bind _yaw (Math|Rotator|BreakRotator _returnvalue))
  (if (> (+ (.Yaw (Math|Rotator|BreakRotator (Transformation|GetWorldRotation (Variables|Default|Getclosed)))) _yaw) 0.0)
    (Transformation|SetWorldRotation _door "0, 0, 0" false false)
    (elif (< (+ (.Yaw (Math|Rotator|BreakRotator (Transformation|GetWorldRotation (Variables|Default|Getopen)))) _yaw) 0.0)
      (Transformation|SetWorldRotation _door "0,-90.000000, 0" false false))))

(fn ConstructionScript)