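; Attic scare actor that reveals red eyes and spawns a Hands actor when the main character's AtticDeath flag is set.
; Tick polls that flag on the player character and, while it is true, turns on the two point light components that form the eyes.
; The SpawnedHands bool acts as a one-shot gate, cleared as Hands spawns 100 units below the actor in its local space.
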(event EventTick
  (params (DeltaSeconds :type Float%20%28single-precision%29))
  (bind _returnvalue (Transformation|GetActorTransform))
  ;[1 1 1] makes the red eyes visble when the player is in attic
  (bind _asmain_char_bp (Utilities|Casting|CastToMainChar_BP (Game|GetPlayerCharacter 0)))
  (if (Variables|/Game/FollowInstructions/Blueprints/MainCharBps/MainChar_BP.MainChar_BP_C|GetAttic_Death _asmain_char_bp)
    (Rendering|SetVisibility (Variables|Default|GetPointLightComponent) true false)
    (if (Variables|Default|GetSpawned_Hands)
      (Variables|Default|SetSpawned_Hands false)
      (Game|SpawnActorfromClass "/Game/FollowInstructions/Blueprints/Attic_Task_BP/Hands.Hands_C" (Math|Transform|MakeTransform (Math|Transform|TransformLocation _returnvalue "0, 0,-100.000000") (Math|Transform|TransformRotation _returnvalue "0, 0, 0")) "Undefined" 0 0))))

(fn ConstructionScript)