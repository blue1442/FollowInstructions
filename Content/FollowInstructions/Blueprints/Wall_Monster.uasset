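; Wall monster trigger actor that builds whispering tension while the player character stays inside its overlap zone.
; Tick raises a per-frame counter while MainChar_BP is inside and lowers it otherwise, scaling the Whispering audio volume with it.
; At the threshold it sets WallMonsterSpawned, mutes the whispers and stops counting; no monster is actually spawned here, only debug prints.
; A disconnected PlaySoundAtLocation node never runs.
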(event EventBeginPlay
  (Variables|Default|SetWallMonsterTimer 0.0))

(event Collision|EventActorBeginOverlap
  (params (OtherActor :type Actor%20Object%20Reference))
  (Utilities|Casting|CastToMainChar_BP OtherActor)
  (Variables|Default|SetIsInTrigger true)
  (Development|PrintString "In Wall Monster thing"))

(event EventTick
  (params (DeltaSeconds :type Float%20%28single-precision%29))
  (bind _wallmonstertimer (Variables|Default|GetWallMonsterTimer))
  (bind _whispering (Variables|Default|GetWhispering))
  (if (not (Variables|Default|GetWallMonsterSpawned))
    (if (Variables|Default|GetIsInTrigger)
      (bind _result (Math|Float|IncrementFloat _wallmonstertimer)
        (:%20%20
          (Development|PrintString (Utilities|String|ToString(Float) _wallmonstertimer) :!label _label)
          (Audio|Components|Audio|AdjustVolume _whispering 0.0 (/ _wallmonstertimer 2.0) :!class /Script/Engine.AudioComponent)
          (if (>= _result 3.6e+02)
            (Development|PrintString "Wall Monster Has Spawned")
            (Variables|Default|SetWallMonsterSpawned true)
            (Audio|Components|Audio|AdjustVolume _whispering 0.0 0.0 :!class /Script/Engine.AudioComponent))))
      (elif (not (< _wallmonstertimer 0.0))
        (Math|Float|DecrementFloat _wallmonstertimer
          (:%20%20
            (goto _label)))))))

(event Collision|EventActorEndOverlap
  (params (OtherActor :type Actor%20Object%20Reference))
  (Utilities|Casting|CastToMainChar_BP OtherActor)
  (Variables|Default|SetIsInTrigger false)
  (Development|PrintString "Out of Wall Monster thing"))

(fn ConstructionScript)