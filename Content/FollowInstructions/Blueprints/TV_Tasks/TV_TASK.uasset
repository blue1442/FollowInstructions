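; TV task actor that puts static on the in-game television and issues a task to the player at minute 32 of each in-game hour.
; Tick watches the character's clock while no task is running; every random branch currently leads to PANIC.
; PANIC plays a voice cue, switches the screen to a camera, flags the player and spawns the Panic Demon AI.
; AVERT and RADIO tasks exist but are disconnected, as is the basement death countdown.
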(event Custom|TV_Task
  ;[1 1 1] Create Static on the TV, choose which task to do
  (Rendering|Material|SetMaterial (Variables|Default|GetTv_screen) 0 "/Game/FollowInstructions/Video/StaticNoiseMaterial.StaticNoiseMaterial")
  (Media|MediaPlayer|OpenSource (Variables|Default|GetTV_MediaPlayer) "/Game/FollowInstructions/Video/tv-static-effect.tv-static-effect")
  (Audio|Components|Audio|SetVolumeMultiplier (Variables|Default|GetTv_Sound) 0.2 :!class /Script/AudioMixer.SynthComponent)
  (switch int (Math|Random|RandomInteger 5)
    (:0
      _)
    (:1
      _)
    (:2
      _)
    (:3
      _)
    (:4
      _)
    (:5
      _))
  (CallFunction|PANIC)
  (Utilities|FlowControl|Delay 1.0)
  (Variables|Default|SetnoTaskRunning true))

(event Custom|PANIC
  ;[1 1 1] Play the Panic Sound
  (Utilities|FlowControl|Delay 5.0)
  (Audio|PlaySoundatLocation "/Game/FollowInstructions/Sounds/Placeholder_PANIC_Voice.Placeholder_PANIC_Voice" (Transformation|GetActorLocation) "0, 0, 0" 1e+01 1.0 0.0 (Variables|Default|GetAttenutation) 0 0)
  (Utilities|FlowControl|Delay 5.0)
  (Rendering|Material|SetMaterial (Variables|Default|GetTv_screen) 0 "/Game/FollowInstructions/House_Assets/Meshes/Custom/camera.camera")
  (Media|MediaPlayer|OpenSource (Variables|Default|GetTV_MediaPlayer) 0)
  (bind _asmain_char_bp (Utilities|Casting|CastToMainChar_BP (Game|GetPlayerCharacter 0)))
  (Variables|/Game/FollowInstructions/Blueprints/MainCharBps/MainChar_BP.MainChar_BP_C|SetTV%20Task%20Run%20 _asmain_char_bp true)
  (Variables|Default|SetBasement_Timer 3e+02)
  (Variables|Default|SetStart_Timer true)
  (AI|SpawnAIFromClass "/Game/FollowInstructions/Blueprints/TV_Tasks/PANIC/PanicDemon.PanicDemon_C" "/Game/FollowInstructions/Blueprints/TV_Tasks/PANIC/PanicBT.PanicBT" "3116.000000,-1202.000000,115.000000" "0, 0, 0" false))

(event Custom|Timer
  ;[1 1 1] Checks to see of teh time is every off-beat hour(8:30, 9:30), then it might start the TV task
  ;;[1 1 1] Timer for the panic demon
)

(event Custom|AVERT
  ;[1 1 1] AVERT Task
  (Utilities|FlowControl|Delay 5.0)
  (Audio|PlaySoundatLocation "/Game/FollowInstructions/Sounds/PH_AVERT.PH_AVERT" (Transformation|GetActorLocation) "0, 0, 0" 1e+01 1.0 0.0 (Variables|Default|GetAttenutation) 0 0)
  (Utilities|FlowControl|Delay 7.0)
  (Rendering|Material|SetMaterial (Variables|Default|GetTv_screen) 0 "/Game/FollowInstructions/House_Assets/Meshes/Custom/camera.camera")
  (Media|MediaPlayer|OpenSource (Variables|Default|GetTV_MediaPlayer) 0)
  (bind _asmain_char_bp (Utilities|Casting|CastToMainChar_BP (Game|GetPlayerCharacter 0)))
  (Utilities|FlowControl|Delay 4.0)
  (Variables|/Game/FollowInstructions/Blueprints/MainCharBps/MainChar_BP.MainChar_BP_C|SetTv%20Task%20Avert _asmain_char_bp true))

(event Custom|RADIO
  ;[1 1 1] RDIO Task
  (Utilities|FlowControl|Delay 5.0)
  (Audio|PlaySoundatLocation "/Game/FollowInstructions/Sounds/PH_AVERT.PH_AVERT" (Transformation|GetActorLocation) "0, 0, 0" 1e+01 1.0 0.0 (Variables|Default|GetAttenutation) 0 0)
  (Utilities|FlowControl|Delay 5.0)
  (Rendering|Material|SetMaterial (Variables|Default|GetTv_screen) 0 "/Game/FollowInstructions/House_Assets/Meshes/Custom/camera.camera")
  (Media|MediaPlayer|OpenSource (Variables|Default|GetTV_MediaPlayer) 0)
  (Utilities|FlowControl|Delay 3.0)
  (if (not (Variables|Default|GetRadio_Playing))
    (bind _returnvalue (Class|MovieSceneTransformOrigin|GetTransformOrigin(Message) (Variables|Default|GetTv_screen)))
    (bind _returnvalue_2 (Game|SpawnActorfromClass "/Game/FollowInstructions/Blueprints/TV_Tasks/RADIO/RADIO.RADIO_C" _returnvalue "Undefined" 0 0))
    (Variables|/Game/FollowInstructions/Blueprints/TV_Tasks/RADIO/RADIO.RADIO_C|SetTv_task _returnvalue_2 self)
    (Variables|Default|SetRadio_Playing true)))

(event EventBeginPlay)

(event Collision|EventActorBeginOverlap
  (params (OtherActor :type Actor%20Object%20Reference)))

(event EventTick
  (params (DeltaSeconds :type Float%20%28single-precision%29))
  ;[1 1 1] Checks to see of teh time is every off-beat hour(8:30, 9:30), then it might start the TV task
  (bind _asfollow_instructions_character (Utilities|Casting|CastToFollowInstructionsCharacter (Game|GetPlayerCharacter 0)))
  (if (Math|Boolean|ANDBoolean (== (Class|KismetMathLibrary|GetMinute (Variables|/Script/FollowInstructions.FollowInstructionsCharacter|GetCurrentDateTime _asfollow_instructions_character)) 32) (== (Math|Random|RandomInteger 0) 0) (Variables|Default|GetnoTaskRunning))
    (Variables|Default|SetnoTaskRunning false)
    (CallFunction|TVTask)))

(fn ConstructionScript)