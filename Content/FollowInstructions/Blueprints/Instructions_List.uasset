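; Instruction list actor that shows pages of instructions on a Cube mesh, which the player can flip through while it is visible.
; BeginPlay registers itself on MainChar_BP and fills an array of page materials.
; Tick mirrors the cube's visibility into a flag that gates input.
; The 2 key and the 1Down action step forward and back through the array with wraparound, swapping the cube's material.
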(event EventBeginPlay
  (bind _material_lists (Variables|Default|GetMaterial_Lists))
  (bind _asmain_char_bp (Utilities|Casting|CastToMainChar_BP (Game|GetPlayerCharacter 0)))
  (Variables|/Game/FollowInstructions/Blueprints/MainChar_BP.MainChar_BP_C|SetinstructionsList _asmain_char_bp self)
  (Utilities|Array|Add _material_lists "/Game/FollowInstructions/Materials/Instructions_list/Lined_Paper.Lined_Paper")
  (Utilities|Array|Add _material_lists "/Game/FollowInstructions/Materials/Instructions_list/Instruction_WordTestM.Instruction_WordTestM")
  (Utilities|Array|Add _material_lists "/Game/FollowInstructions/Materials/Instructions_list/Instruction_WordtestM2.Instruction_WordtestM2"))

(event Collision|EventActorBeginOverlap
  (params (OtherActor :type Actor%20Object%20Reference)))

(event EventTick
  (params (DeltaSeconds :type Float%20%28single-precision%29))
  (if (Rendering|IsVisible (Variables|Default|GetCube))
    (Variables|Default|SetIfVisible true)
    (else
      (Variables|Default|SetIfVisible false))))

(event Input|ActionEvents|InputAction1Down
  (params (Key :type Key%20Structure))
  (bind _material_lists (Variables|Default|GetMaterial_Lists))
  ;[1 1 1] Changes the Pages of the instructions back and forth
  (:Pressed
    (if (Variables|Default|GetIfVisible)
      (Math|Integer|DecrementInt (Variables|Default|GetCurrent_PageIndex)
        (:%20%20
          (if (< (Variables|Default|GetCurrent_PageIndex) 0)
            (Variables|Default|SetCurrent_PageIndex (Utilities|Array|LastIndex _material_lists)))
          (Rendering|Material|SetMaterial (Variables|Default|GetCube) 0 (Utilities|Array|Get(acopy) _material_lists (Variables|Default|GetCurrent_PageIndex))))))))

(event Input|KeyboardEvents|2
  (params (Key :type Key%20Structure))
  (bind _material_lists (Variables|Default|GetMaterial_Lists))
  ;[1 1 1] Changes the Pages of the instructions back and forth
  (:Pressed
    (if (Variables|Default|GetIfVisible)
      (Math|Integer|IncrementInt (Variables|Default|GetCurrent_PageIndex)
        (:%20%20
          (if (> (Variables|Default|GetCurrent_PageIndex) (Utilities|Array|LastIndex _material_lists))
            (Variables|Default|SetCurrent_PageIndex 0))
          (Rendering|Material|SetMaterial (Variables|Default|GetCube) 0 (Utilities|Array|Get(acopy) _material_lists (Variables|Default|GetCurrent_PageIndex))))))))

(fn ConstructionScript)