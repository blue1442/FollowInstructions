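; Scittering Sound is a hazard actor that chases the player during the grandfather clock task and ends the run on contact.
; While the character's GrandfatherClockRun flag is set, Tick calls MoveComponentTo toward the player, scaling duration by distance for a roughly constant speed.
; When the flag is clear, the actor destroys itself.
; A Box overlap with the player prints a bathroom failure message and opens Death_level.
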(event OnComponentBeginOverlap(Box)
  (params (OverlappedComponent :type Primitive%20Component%20Object%20Reference) (OtherActor :type Actor%20Object%20Reference) (OtherComp :type Primitive%20Component%20Object%20Reference) (OtherBodyIndex :type Integer) (bFromSweep :type Boolean) (SweepResult :type Hit%20Result%20Structure%20%28by%20ref%29))
  ;[1 1 1] kills the player when the sounds overlaps them
  (bind _asmain_char_bp (Utilities|Casting|CastToMainChar_BP (Game|GetPlayerCharacter 0)))
  (if (== _asmain_char_bp OtherActor)
    (Development|PrintString "You didnt go to the bathroom fast enough")
    (Game|OpenLevel(byName) "Death_level")))

(event EventTick
  (params (DeltaSeconds :type Float%20%28single-precision%29))
  ;[1 1 1] Moves the sound towards the player when appropriate, otherwise destroys the sound
  (bind _asmain_char_bp (Utilities|Casting|CastToMainChar_BP (Game|GetPlayerCharacter 0)))
  (if (Variables|/Game/FollowInstructions/Blueprints/MainCharBps/MainChar_BP.MainChar_BP_C|GetGrandfather_Clock_run _asmain_char_bp)
    (bind _asmain_char_bp_2 (Utilities|Casting|CastToMainChar_BP (Game|GetPlayerCharacter 0)))
    (Components|MoveComponentTo (Variables|Default|GetDefaultSceneRoot) (Transformation|GetWorldLocation (Variables|/Script/Engine.Actor|GetRootComponent _asmain_char_bp_2)) "0, 0, 0" false false (/ (Math|Vector|Distance(Vector) (Transformation|GetWorldLocation (Variables|/Script/Engine.Actor|GetRootComponent _asmain_char_bp_2)) (Transformation|GetWorldLocation (Variables|Default|GetDefaultSceneRoot))) 2.5e+02) false)
    (else
      (Actor|DestroyActor))))

(fn ConstructionScript)