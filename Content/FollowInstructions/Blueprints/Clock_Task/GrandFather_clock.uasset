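; Grandfather clock that chimes the hour count whenever the player character's in-game time reaches minute zero.
; Tick triggers a delayed-loop macro that plays spaced, attenuated chimes, with Safeguard blocking retriggers until it completes.
; At eight o'clock, RandomizeChimes can add a chime; its decrement branch is unreachable with RandomInteger(2).
; A wrong count sets GrandfatherClockRun on MainChar_BP and spawns Scittering_Sound at a fixed location after chiming.
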(event Custom|Clock%20Chime
  (params (lastIndex :type Integer))
  ;[1 1 1] manages the clock chimes
  (bind _output_get (Variables|Default|SetchimesUsed lastIndex))
  ;;[1 1 1] Make sure the clock chimes on an interval
  (Utilities|ForLoopwithDelay 1 _output_get :!label _label
    (:Loop%20Body
      (Audio|PlaySoundatLocation "/Game/FollowInstructions/Sounds/Chime.Chime" (Transformation|GetWorldLocation (Variables|Default|GetStaticMeshComponent1)) "0, 0, 0" 1.0 1.0 0.0 (Variables|Default|GetFalloff) 0 0))
    (:Completed
      (Variables|Default|SetSafeguard true)
      (if (!= (Variables|Default|GetTemp_time) (Variables|Default|GetchimesUsed))
        (bind _asmain_char_bp (Utilities|Casting|CastToMainChar_BP (Game|GetPlayerCharacter 0)))
        (Variables|/Game/FollowInstructions/Blueprints/MainCharBps/MainChar_BP.MainChar_BP_C|SetGrandfather_Clock_run _asmain_char_bp true)
        (Game|SpawnActorfromClass "/Game/FollowInstructions/Blueprints/Clock_Task/Scittering_Sound.Scittering_Sound_C" (Math|Transform|MakeTransform "2530.000000,-3480.000000,20.000000") "Undefined" 0 0)))
    (:Delay%20Out
      (Utilities|FlowControl|Delay 1.168)
      (goto _label Delay%20In))))

(event EventTick
  (params (DeltaSeconds :type Float%20%28single-precision%29))
  ;[1 1 1] Gets the current game time mod interval, returns true if ture
  (bind _asfollow_instructions_character (Utilities|Casting|CastToFollowInstructionsCharacter (Game|GetPlayerCharacter 0)))
  (if (and (Variables|Default|GetSafeguard) (== (Class|KismetMathLibrary|GetMinute (Variables|/Script/FollowInstructions.FollowInstructionsCharacter|GetCurrentDateTime _asfollow_instructions_character)) 0))
    (Variables|Default|SetSafeguard false)
    (Variables|Default|SetTemp_time (Class|KismetMathLibrary|GetHour12 (Variables|/Script/FollowInstructions.FollowInstructionsCharacter|GetCurrentDateTime _asfollow_instructions_character)))
    (bind _output_get (Variables|Default|SetInteration_Count (Class|KismetMathLibrary|GetHour12 (Variables|/Script/FollowInstructions.FollowInstructionsCharacter|GetCurrentDateTime _asfollow_instructions_character))))
    ;;[1 1 1] If the Hour is set to X, then run the random chime function
    (if (== _output_get 8)
      (CallFunction|RandomizeChimes))
    (CallFunction|ClockChime _output_get)))

(fn ConstructionScript)

(fn RandomizeChimes
  (switch int (Math|Random|RandomInteger 2)
    (:0
      (bind _result (Math|Integer|IncrementInt (Variables|Default|GetInteration_Count))
        (:%20%20
          (Variables|Default|SetInteration_Count _result))))
    (:2
      (bind _result_2 (Math|Integer|DecrementInt (Variables|Default|GetInteration_Count))
        (:%20%20
          (Variables|Default|SetInteration_Count _result_2))))))