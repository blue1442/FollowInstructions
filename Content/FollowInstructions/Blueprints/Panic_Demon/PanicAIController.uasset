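; AI controller for the Panic Demon enemy that starts its behavior tree and gives it the player as a target.
; On BeginPlay it sets up the PanicBB blackboard, stores the player character under PlayerObj and runs PanicBT.
; Each tick it casts its PanicDemon reference and, while CaughtPlayer is true, calls UseBlackboard with no asset specified.
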(event EventBeginPlay
  (bind _blackboardcomponent (Class|AIController|UseBlackboard "/Game/FollowInstructions/Blueprints/Panic_Demon/PanicBB.PanicBB"))
  (AI|Components|Blackboard|SetValueasObject _blackboardcomponent (Variables|Default|GetPlayerObj) (Game|GetPlayerCharacter 0))
  (AI|RunBehaviorTree "/Game/FollowInstructions/Blueprints/Panic_Demon/PanicBT.PanicBT"))

(event EventTick
  (params (DeltaSeconds :type Float%20%28single-precision%29))
  (bind _aspanic_demon (Utilities|Casting|CastToPanicDemon (Variables|Default|GetPanicDemon)))
  (if (Variables|/Game/FollowInstructions/Blueprints/Panic_Demon/PanicDemon.PanicDemon_C|GetCaughtPlayer _aspanic_demon)
    (Class|AIController|UseBlackboard)))

(fn ConstructionScript)