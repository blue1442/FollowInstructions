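; Grandfather clock actor that plays a series of spatialized chimes at BeginPlay, starting from a base count of five.
; ClockChime passes the count through RandomizeChimes, which may increment it; the decrement case is unreachable with RandomInteger(2).
; A custom ForLoopWithDelay macro spaces the chime sounds at the clock mesh's location.
; On completion, it prints a danger message if the chime count differs from the intended one.
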(event Custom|Clock%20Chime
  (params (lastIndex :type Integer))
  (Variables|Default|SetchimesUsed lastIndex)
  (CallFunction|RandomizeChimes)
  (Utilities|ForLoopwithDelay 1 (Variables|Default|GetchimesUsed) false 1.168
    (:LoopBody
      (Audio|PlaySoundatLocation "/Game/FollowInstructions/Sounds/Chime.Chime" (Transformation|GetWorldLocation (Variables|Default|GetStaticMeshComponent1)) "0, 0, 0" 1.0 1.0 0.0 (Variables|Default|GetFalloff) 0 0))
    (:Completed
      (if (!= (Variables|Default|GetInteration_Count) (Variables|Default|GetchimesUsed))
        (Development|PrintString "I'm in danger")))))

(event Collision|EventActorBeginOverlap
  (params (OtherActor :type Actor%20Object%20Reference)))

(event EventTick
  (params (DeltaSeconds :type Float%20%28single-precision%29)))

(event EventBeginPlay
  (bind _output_get (Variables|Default|SetInteration_Count 5))
  (CallFunction|ClockChime _output_get))

(fn ConstructionScript)

(fn RandomizeChimes
  (switch int (Math|Random|RandomInteger 2)
    (:0
      (bind _result (Math|Integer|IncrementInt (Variables|Default|GetchimesUsed))
        (:%20%20
          (Variables|Default|SetchimesUsed _result))))
    (:2
      (bind _result_2 (Math|Integer|DecrementInt (Variables|Default|GetchimesUsed))
        (:%20%20
          (Variables|Default|SetchimesUsed _result_2))))))