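; TV task actor that stages a panic event on a television, with a countdown toward a panic death.
; Tick calls the TV task whenever the player character's in-game minute is 32; every random branch leads to it.
; The task shows static, plays a delayed panic voice, then switches to a camera material and enables the countdown.
; The Timer event decrements BasementTimer while enabled, setting PanicDeath at zero.
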(event Custom|TV_Task
  ;[1 1 1] Create Static on the TV, choose which task to do
  (Rendering|Material|SetMaterial (Variables|Default|GetTv_screen) 0 "/Game/FollowInstructions/Video/StaticNoiseMaterial.StaticNoiseMaterial")
  (Media|MediaPlayer|OpenSource (Variables|Default|GetTV_MediaPlayer) "/Game/FollowInstructions/Video/tv-static-effect.tv-static-effect")
  (Audio|Components|Audio|SetVolumeMultiplier (Variables|Default|GetTv_Sound) 0.2 :!class /Script/AudioMixer.SynthComponent)
  (CallFunction|PANIC))

(event Custom|PANIC
  ;[1 1 1] Play the Panic Sound
  (Utilities|FlowControl|Delay 5.0)
  (Audio|PlaySoundatLocation "/Game/FollowInstructions/Sounds/Placeholder_PANIC_Voice.Placeholder_PANIC_Voice" "0, 0, 0" "0, 0, 0" 1e+01 1.0 0.0 (Variables|Default|GetAttenutation) 0 0)
  (Utilities|FlowControl|Delay 5.0)
  (Rendering|Material|SetMaterial (Variables|Default|GetTv_screen) 0 "/Game/FollowInstructions/House_Assets/Meshes/Custom/camera.camera")
  (Media|MediaPlayer|OpenSource (Variables|Default|GetTV_MediaPlayer) 0)
  (Variables|Default|SetStart_Timer true))

(event Custom|Timer
  (bind _basement_timer (Variables|Default|GetBasement_Timer))
  ;[1 1 1] Checks to see of teh time is every off-beat hour(8:30, 9:30), then it might start the TV task
  (if (Variables|Default|GetStart_Timer)
    (Math|Float|DecrementFloat _basement_timer
      (:%20%20
        (if (== _basement_timer 0.0)
          (Variables|Default|SetPanic_Death true))))))

(event EventBeginPlay)

(event Collision|EventActorBeginOverlap
  (params (OtherActor :type Actor%20Object%20Reference)))

(event EventTick
  (params (DeltaSeconds :type Float%20%28single-precision%29))
  ;[1 1 1] Checks to see of teh time is every off-beat hour(8:30, 9:30), then it might start the TV task
  (bind _asfollow_instructions_character (Utilities|Casting|CastToFollowInstructionsCharacter (Game|GetPlayerCharacter 0)))
  (if (== (Class|KismetMathLibrary|GetMinute (Variables|/Script/FollowInstructions.FollowInstructionsCharacter|GetCurrentDateTime _asfollow_instructions_character)) 32)
    (switch int (Math|Random|RandomInteger 2)
      (:0
        _)
      (:1
        _)
      (:2
        _))
    (CallFunction|TVTask)))

(fn ConstructionScript)