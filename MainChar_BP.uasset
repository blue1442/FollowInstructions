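; Player character Blueprint with mouse look and two-stage physics object pickup on the left mouse button.
; A camera line trace grabs the hit component with a PhysicsHandle, holding it in front until button release stows it at HeldItemLocation with collision ignored.
; The next press brings it back in front with world collision, and releasing drops it.
; Look axis events, rather than Tick, update the handle's target.
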(event EventBeginPlay
  (Variables|Default|SetbUseControllerRotationYaw true))

(event Collision|EventActorBeginOverlap
  (params (OtherActor :type Actor%20Object%20Reference)))

(event EventTick
  (params (DeltaSeconds :type Float%20%28single-precision%29)))

(event Input|AxisEvents|InputAxisTurnRight
  (params (AxisValue :type Float%20%28single-precision%29))
  (bind _playercamera (Variables|Default|GetPlayerCamera))
  (bind _physicshandle (Variables|Default|GetPhysicsHandle))
  ;[1 1 1] keeps pickup up object in front of player
  (Pawn|Input|AddControllerYawInput AxisValue)
  (if (Variables|Default|GetobjectInFront)
    (Physics|Components|PhysicsHandle|SetTargetLocation _physicshandle (+ (Transformation|GetWorldLocation _playercamera) (* (Math|Vector|GetForwardVector _playercamera) 1e+02)))
    (else
      (Class|PhysicsHandleComponent|SetTargetLocationandRotation _physicshandle (Transformation|GetWorldLocation (Variables|Default|GetheldItemLocation)) "0, 0, 0"))))

(event Input|AxisEvents|InputAxisLookUp
  (params (AxisValue :type Float%20%28single-precision%29))
  (bind _playercamera (Variables|Default|GetPlayerCamera))
  (bind _physicshandle (Variables|Default|GetPhysicsHandle))
  ;[1 1 1] keeps pickup up object in front of player
  (Pawn|Input|AddControllerPitchInput AxisValue)
  (if (Variables|Default|GetobjectInFront)
    (Physics|Components|PhysicsHandle|SetTargetLocation _physicshandle (+ (Transformation|GetWorldLocation _playercamera) (* (Math|Vector|GetForwardVector _playercamera) 1e+02)))
    (else
      (Class|PhysicsHandleComponent|SetTargetLocationandRotation _physicshandle (Transformation|GetWorldLocation (Variables|Default|GetheldItemLocation)) "0, 0, 0"))))

(event Input|MouseEvents|LeftMouseButton
  (params (Key :type Key%20Structure))
  (bind _playercamera (Variables|Default|GetPlayerCamera))
  (bind _returnvalue (Transformation|GetWorldLocation _playercamera))
  (:Pressed
    ;[1 1 1] handles picking up object
    (if (== (Variables|Default|GetheldObject) 0)
      (bind _outhit (Collision|LineTraceByChannel _returnvalue (+ _returnvalue (* (Math|Vector|GetForwardVector _playercamera) 1.5e+02)) "TraceTypeQuery1" false 0 "ForDuration" true "(R=0.000000,G=1.000000,B=0.074661,A=1.000000)" "(R=1.000000,G=0.155322,B=0.000000,A=1.000000)"))
      (if (.bBlockingHit (Collision|BreakHitResult _outhit))
        (Collision|SetCollisionResponsetoChannel (.HitComponent (Collision|BreakHitResult _outhit)) "ECC_Pawn" "ECR_Ignore")
        (Class|PhysicsHandleComponent|GrabComponentatLocation (Variables|Default|GetPhysicsHandle) (.HitComponent (Collision|BreakHitResult _outhit)) "None" (Transformation|GetWorldLocation (.HitComponent (Collision|BreakHitResult _outhit))))
        (Variables|Default|SetobjectInFront true :!label _label))
      (else
        (Collision|SetCollisionResponsetoChannel (.HitComponent (Collision|BreakHitResult _outhit)) "ECC_WorldStatic" "ECR_Block")
        (Collision|SetCollisionResponsetoChannel (.HitComponent (Collision|BreakHitResult _outhit)) "ECC_WorldDynamic" "ECR_Block")
        (goto _label))))
  (:Released
    (if (== (Variables|Default|GetheldObject) 0)
      (Variables|Default|SetobjectInFront false)
      (bind _output_get (Variables|Default|SetheldObject (.HitComponent (Collision|BreakHitResult _outhit))))
      (if (!= _output_get 0)
        (Collision|SetCollisionResponsetoAllChannels (.HitComponent (Collision|BreakHitResult _outhit)) "ECR_Ignore"))
      (else
        (Physics|Components|PhysicsHandle|ReleaseComponent (Variables|Default|GetPhysicsHandle))
        (Variables|Default|SetheldObject 0)
        (Collision|SetCollisionResponsetoAllChannels (.HitComponent (Collision|BreakHitResult _outhit)) "ECR_Block")
        (Variables|Default|SetobjectInFront false)))))

(fn ConstructionScript)